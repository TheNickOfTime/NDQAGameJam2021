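; Interactable research terminal that toggles a computer UI, halting player movement while it is open.
; Jump presses move one player resource into the game mode's research total with a sound, or play a denied sound when none remain.
; Each transfer updates the UI counters and fill bar, flagging a win on the player HUD at full research.
; Jump does not check whether the UI is open, and timed-transfer logic is left unconnected.
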(event EventTick
  (params (DeltaSeconds :type Float%20%28single-precision%29)))

(event EventBeginPlay
  (bind _returnvalue (Game|GetGameMode))
  (bind _asbase_mode (Utilities|Casting|CastToBaseMode _returnvalue))
  (|CallParentFunction)
  (bind _returnvalue_2 (UserInterface|CreateWidget "/Game/Blueprints/UI/ComputerUI.ComputerUI_C" (Game|GetPlayerController 0)))
  (bind _output_get (Variables|Default|SetUI _returnvalue_2))
  (Utilities|FlowControl|Delay 0.0)
  (Variables|/Game/Blueprints/UI/ComputerUI.ComputerUI_C|SetFillPercent _output_get (/ (Variables|/Game/Blueprints/Modes/BaseMode.BaseMode_C|GetCurrentResearch _asbase_mode) (Variables|/Game/Blueprints/Modes/BaseMode.BaseMode_C|GetMaxResearch _asbase_mode))))

(event Input|ActionEvents|InputActionJump
  (params (Key :type Key%20Structure :default "None"))
  (bind _returnvalue (Game|GetPlayerCharacter 0))
  (bind _returnvalue_2 (Game|GetGameMode))
  (bind _ui (Variables|Default|GetUI))
  (bind _asplayer (Utilities|Casting|CastToPlayer _returnvalue))
  (bind _asbase_mode (Utilities|Casting|CastToBaseMode _returnvalue_2))
  (bind _currentresource (Variables|/Game/Blueprints/Player/Player.Player_C|GetCurrentResource _asplayer))
  (bind _currentresearch (Variables|/Game/Blueprints/Modes/BaseMode.BaseMode_C|GetCurrentResearch _asbase_mode))
  (:Pressed
    (if (> _currentresource 0)
      (Audio|PlaySound2D "/Game/Audio/SFX/UI_Nav_Blips/UI_Blips_High.UI_Blips_High" 1.0 1.0 0.0 0 0)
      (bind _result (Math|Integer|DecrementInt _currentresource)
        (:%20%20
          (Variables|/Game/Blueprints/UI/ComputerUI.ComputerUI_C|SetResourceA _ui _result)
          (bind _result_2 (Math|Float|IncrementFloat _currentresearch)
            (:%20%20
              (Variables|/Game/Blueprints/UI/ComputerUI.ComputerUI_C|SetResourceB _ui (Math|Float|Truncate _result_2))
              (bind _output_get (Variables|/Game/Blueprints/UI/ComputerUI.ComputerUI_C|SetFillPercent _ui (/ _currentresearch (Variables|/Game/Blueprints/Modes/BaseMode.BaseMode_C|GetMaxResearch _asbase_mode))))
              (if (>= _output_get 1.0)
                (Variables|/Game/Blueprints/UI/HUD.HUD_C|SetIsWin (Variables|/Game/Blueprints/Player/Player.Player_C|GetHUD (.AsPlayer (Utilities|Casting|CastToPlayer (Game|GetPlayerCharacter 0)))) true))))))
      (else
        (Audio|PlaySound2D "/Game/Audio/SFX/Denied_UI.Denied_UI" 1.0 1.0 0.0 0 0)))))

(fn ConstructionScript
  (|CallParentFunction))

(fn OnInteract
  (bind _returnvalue (Game|GetPlayerController 0))
  (bind _returnvalue_2 (Game|GetPlayerCharacter 0))
  (bind _ui (Variables|Default|GetUI))
  (bind _ui_2 (Variables|Default|GetUI))
  (bind _charactermovement (Variables|/Script/Engine.Character|GetCharacterMovement _returnvalue_2))
  (Variables|Default|SetInUI (not (Variables|Default|GetInUI)))
  (if (Variables|Default|GetInUI)
    (UserInterface|Viewport|AddtoViewport _ui 0)
    (Components|Activation|Deactivate _charactermovement)
    (Variables|/Game/Blueprints/UI/ComputerUI.ComputerUI_C|SetResourceA _ui_2 (Variables|/Game/Blueprints/Player/Player.Player_C|GetCurrentResource (.AsPlayer (Utilities|Casting|CastToPlayer (Game|GetPlayerCharacter 0)))))
    (Variables|/Game/Blueprints/UI/ComputerUI.ComputerUI_C|SetResourceB _ui_2 (Math|Float|Truncate (Variables|/Game/Blueprints/Modes/BaseMode.BaseMode_C|GetCurrentResearch (.AsBase%20Mode (Utilities|Casting|CastToBaseMode (Game|GetGameMode))))))
    (else
      (Widget|RemovefromParent _ui)
      (Input|EnableInput _returnvalue _returnvalue)
      (Components|Activation|Activate _charactermovement false))))