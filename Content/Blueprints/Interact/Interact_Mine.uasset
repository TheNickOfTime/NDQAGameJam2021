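; Interactable mine that toggles a trigger-rumble minigame, freezing player movement while active, and spawns a resource on completion.
; Each trigger axis is scored against a random goal through RumbleMath, with dynamic force feedback signalling closeness.
; Tick raises progress while both triggers pass their thresholds, otherwise drains it, and drives audio pitch and RumbleUI colors.
; Full progress disables further interaction, plays a success sound and destroys the mine.
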(event Custom|StopRumble
  (bind _returnvalue (Game|GetPlayerController 0))
  (Utilities|FlowControl|Sequence
    (:then_0
      (Game|Feedback|PlayDynamicForceFeedback _returnvalue (stale Input|AxisEvents|InputAxisLeftTrigger _output_get_2) -1.0 (stale Input|AxisEvents|InputAxisLeftTrigger _output_get_3) (not (stale Input|AxisEvents|InputAxisLeftTrigger _output_get_3)) false false) ; enters at Stop
    )
    (:then_1
      (Game|Feedback|PlayDynamicForceFeedback _returnvalue (stale Input|AxisEvents|InputAxisRightTrigger _output_get_2) -1.0 false false (stale Input|AxisEvents|InputAxisRightTrigger _output_get_3) (not (stale Input|AxisEvents|InputAxisRightTrigger _output_get_3))) ; enters at Stop
    )))

(event EventTick
  (params (DeltaSeconds :type Float%20%28single-precision%29))
  (bind _ui (Variables|Default|GetUI))
  (if (Variables|Default|GetInMinigame)
    (Utilities|FlowControl|Sequence
      (:then_0
        ;[1 1 1] Set Progress
        (Variables|Default|SetProgressCurrent (Math|Float|Clamp(Float) (+ (Variables|Default|GetProgressCurrent) (* (Utilities|Time|GetWorldDeltaSeconds) (select (and (Variables|Default|GetLeftThreshold) (Variables|Default|GetRightThreshold)) 1.0 -1.0))) 0.0 (Variables|Default|GetProgressMax)))
        (Audio|Components|Audio|SetPitchMultiplier (Variables|Default|GetAudio) (Math|Float|Lerp 0.5 1.0 (* (Variables|Default|GetRightValue) (Variables|Default|GetLeftValue)))))
      (:then_1
        ;[1 1 1] Update UI
        (Variables|/Game/Blueprints/UI/RumbleUI.RumbleUI_C|SetColor1 _ui (Variables|Default|GetLeftValue))
        (Variables|/Game/Blueprints/UI/RumbleUI.RumbleUI_C|SetColor2 _ui (Variables|Default|GetRightValue))
        (Variables|/Game/Blueprints/UI/RumbleUI.RumbleUI_C|SetColor3 _ui (/ (Variables|Default|GetProgressCurrent) (Variables|Default|GetProgressMax))))
      (:then_2
        (if (>= (Variables|Default|GetProgressCurrent) (Variables|Default|GetProgressMax))
          (CallFunction|OnComplete)
          (CallFunction|StopRumble)
          (Audio|PlaySoundatLocation "/Game/Audio/SFX/MiniGame_Success.MiniGame_Success" (Transformation|GetActorLocation) "0, 0, 0" 1.0 1.0 0.0 0 0 0))))))

(event EventBeginPlay
  (|CallParentFunction)
  (bind _returnvalue (UserInterface|CreateWidget "/Game/Blueprints/UI/RumbleUI.RumbleUI_C" (Game|GetPlayerController 0)))
  (Variables|Default|SetUI _returnvalue)
  (Variables|Default|SetLeftTriggerGoal (Math|Random|RandomFloatinRange 0.0 1.0))
  (Variables|Default|SetRightTriggerGoal (Math|Random|RandomFloatinRange 0.0 1.0))
  (Transformation|SetActorRotation "0, 0, 0")
  (Audio|Components|Audio|SetPitchMultiplier (Variables|Default|GetAudio) 0.5))

(event Input|AxisEvents|InputAxisLeftTrigger
  (params (AxisValue :type Float%20%28single-precision%29))
  (if (Variables|Default|GetInMinigame)
    (bind _output_get (Variables|Default|SetLeftTriggerCurrent AxisValue))
    (bind _output_get_2 (Variables|Default|SetLeftValue (.Value (Utilities|RumbleMath _output_get (Variables|Default|GetLeftTriggerGoal)))))
    (bind _output_get_3 (Variables|Default|SetLeftThreshold (.Passed%20Threshold (Utilities|RumbleMath _output_get (Variables|Default|GetLeftTriggerGoal)))))
    (Game|Feedback|PlayDynamicForceFeedback (Game|GetPlayerController 0) _output_get_2 -1.0 _output_get_3 (not _output_get_3) false false)))

(event Input|AxisEvents|InputAxisRightTrigger
  (params (AxisValue :type Float%20%28single-precision%29))
  (if (Variables|Default|GetInMinigame)
    (bind _output_get (Variables|Default|SetRightTriggerCurrent AxisValue))
    (bind _output_get_2 (Variables|Default|SetRightValue (.Value (Utilities|RumbleMath _output_get (Variables|Default|GetRightTriggerGoal)))))
    (bind _output_get_3 (Variables|Default|SetRightThreshold (.Passed%20Threshold (Utilities|RumbleMath _output_get (Variables|Default|GetRightTriggerGoal)))))
    (Game|Feedback|PlayDynamicForceFeedback (Game|GetPlayerController 0) _output_get_2 -1.0 false false _output_get_3 (not _output_get_3))))

(fn ConstructionScript
  (|CallParentFunction))

(fn OnInteract
  (bind _returnvalue (Game|GetPlayerCharacter 0))
  (bind _ui (Variables|Default|GetUI))
  (bind _audio (Variables|Default|GetAudio))
  (bind _charactermovement (Variables|/Script/Engine.Character|GetCharacterMovement _returnvalue))
  (if (not (Variables|Default|GetIsComplete))
    (bind _output_get (Variables|Default|SetInMinigame (not (Variables|Default|GetInMinigame))))
    (if _output_get
      (UserInterface|Viewport|AddtoViewport _ui 0)
      (Components|Activation|Deactivate _charactermovement)
      (Audio|Components|Audio|Play _audio 0.0)
      (else
        (Widget|RemovefromParent _ui)
        (Components|Activation|Activate _charactermovement false)
        (Audio|Components|Audio|Stop _audio)))))

(fn SpawnResource
  (Game|SpawnActorfromClass "/Game/Blueprints/Interact/Interact_Resource.Interact_Resource_C" (Math|Conversions|ToTransform(Vector) (Transformation|GetActorLocation)) "Undefined" 0 0)
  (Actor|DestroyActor))

(fn OnComplete
  (CallFunction|OnInteract)
  (Variables|Default|SetIsComplete true)
  (Components|Sphere|SetSphereRadius (Variables|Default|GetActivationRadius) 0.0 true)
  (Components|Sphere|SetSphereRadius (Variables|Default|GetInteractRadius) 0.0 true)
  (CallFunction|SetPrompt false false)
  (CallFunction|SpawnResource))