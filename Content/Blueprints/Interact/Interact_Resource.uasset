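; Collectible resource pickup that moves toward the player and adds one to their resource count when interacted with.
; The interact radius starts at zero and is set to its configured size once the physics sphere comes to rest.
; While the activation radius is triggered, Tick lerps the actor toward the player at a speed scaled by frame time.
; Interacting increments the Player's CurrentResource, prints it and destroys the pickup.
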(event EventTick
  (params (DeltaSeconds :type Float%20%28single-precision%29))
  (Utilities|FlowControl|Sequence
    (:then_0
      (|Waittohitground))
    (:then_1
      (if (Variables|Default|GetMoveToPlayer)
        (Transformation|SetActorLocation (Math|Vector|Lerp(Vector) (Transformation|GetActorLocation) (Transformation|GetActorLocation (Game|GetPlayerCharacter 0)) (* DeltaSeconds (Variables|Default|GetMoveSpeed))) false false)))))

(event EventBeginPlay
  (Components|Sphere|SetSphereRadius (Variables|Default|GetInteractRadius) 0.0 false)
  (Components|Sphere|SetSphereRadius (Variables|Default|GetActivationRadius) 5e+02 true))

(fn ConstructionScript
  (|CallParentFunction))

(fn OnInteract
  (bind _asplayer (Utilities|Casting|CastToPlayer (Game|GetPlayerCharacter 0)))
  (bind _result (Math|Integer|IncrementInt (Variables|/Game/Blueprints/Player/Player.Player_C|GetCurrentResource _asplayer))
    (:%20%20
      (Development|PrintString (Utilities|String|ToString(Integer) _result))
      (Actor|DestroyActor))))

(fn OnEnterActivation
  (Variables|Default|SetMoveToPlayer true))

(fn OnExitActivation
  (Variables|Default|SetMoveToPlayer false))