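; Base interactable Blueprint with a placeholder OnInteract for specific behavior, triggered on overlap when no input is required.
; Construction sizes two spheres from Radius, collapsing the larger activation sphere to zero when input is not required.
; With input required, the outer sphere shows the ButtonPrompt widget's image.
; The inner sphere adds its text, sets CanInteract and registers itself as the Player's CurrentInteract, clearing both on exit.
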(event OnComponentBeginOverlap(ActivationRadius)
  (params (OverlappedComponent :type Primitive%20Component%20Object%20Reference) (OtherActor :type Actor%20Object%20Reference) (OtherComp :type Primitive%20Component%20Object%20Reference) (OtherBodyIndex :type Integer) (bFromSweep :type Boolean) (SweepResult :type Hit%20Result%20Structure%20%28by%20ref%29))
  (if (== OtherActor (Game|Player|GetPlayerPawn 0))
    (CallFunction|OnEnterActivation)))

(event OnComponentEndOverlap(ActivationRadius)
  (params (OverlappedComponent :type Primitive%20Component%20Object%20Reference) (OtherActor :type Actor%20Object%20Reference) (OtherComp :type Primitive%20Component%20Object%20Reference) (OtherBodyIndex :type Integer))
  (if (== OtherActor (Game|Player|GetPlayerPawn 0))
    (CallFunction|OnExitActivation)))

(event OnComponentBeginOverlap(InteractRadius)
  (params (OverlappedComponent :type Primitive%20Component%20Object%20Reference) (OtherActor :type Actor%20Object%20Reference) (OtherComp :type Primitive%20Component%20Object%20Reference) (OtherBodyIndex :type Integer) (bFromSweep :type Boolean) (SweepResult :type Hit%20Result%20Structure%20%28by%20ref%29))
  (if (== OtherActor (Game|Player|GetPlayerPawn 0))
    (CallFunction|OnEnterInteract)))

(event OnComponentEndOverlap(InteractRadius)
  (params (OverlappedComponent :type Primitive%20Component%20Object%20Reference) (OtherActor :type Actor%20Object%20Reference) (OtherComp :type Primitive%20Component%20Object%20Reference) (OtherBodyIndex :type Integer))
  (if (== OtherActor (Game|Player|GetPlayerPawn 0))
    (CallFunction|OnExitInteract)))

(event EventBeginPlay
  (bind _asbutton_prompt (Utilities|Casting|CastToButtonPrompt (UserInterface|GetWidget (Variables|Default|GetPrompt))))
  (Rendering|Components|TextRender|SetText (Variables|/Game/Blueprints/UI/ButtonPrompt.ButtonPrompt_C|GetTextBlock_52 _asbutton_prompt) (Variables|Default|GetInteractText)))

(fn ConstructionScript
  (bind _radius (Variables|Default|GetRadius))
  (Components|Sphere|SetSphereRadius (Variables|Default|GetInteractRadius) _radius true)
  (Components|Sphere|SetSphereRadius (Variables|Default|GetActivationRadius) (Math|Float|SelectFloat (+ _radius 1.5e+02) 0.0 (Variables|Default|GetRequiresInput)) true))

(fn OnInteract
  (Development|PrintString "You have not implimented specific interact functionality"))

(fn OnEnterActivation
  (if (Variables|Default|GetRequiresInput)
    (CallFunction|SetPrompt true false)))

(fn OnExitActivation
  (if (Variables|Default|GetRequiresInput)
    (CallFunction|SetPrompt false false)))

(fn OnEnterInteract
  (if (Variables|Default|GetRequiresInput)
    (CallFunction|SetPrompt true true)
    (Variables|Default|SetCanInteract true)
    (bind _asplayer (Utilities|Casting|CastToPlayer (Game|GetPlayerCharacter 0)))
    (Variables|/Game/Blueprints/Player/Player.Player_C|SetCurrentInteract _asplayer self)
    (else
      (CallFunction|OnInteract))))

(fn OnExitInteract
  (if (Variables|Default|GetRequiresInput)
    (CallFunction|SetPrompt true false)
    (Variables|Default|SetCanInteract false)
    (bind _asplayer (Utilities|Casting|CastToPlayer (Game|GetPlayerCharacter 0)))
    (Variables|/Game/Blueprints/Player/Player.Player_C|SetCurrentInteract _asplayer 0)))

(fn SetPrompt
  (params (IsVisible :type Boolean) (IsInteract :type Boolean))
  (bind _asbutton_prompt (Utilities|Casting|CastToButtonPrompt (UserInterface|GetWidget (Variables|Default|GetPrompt))))
  (Widget|SetVisibility (Variables|/Game/Blueprints/UI/ButtonPrompt.ButtonPrompt_C|GetImage_0 _asbutton_prompt) (select IsVisible "Visible" "Collapsed"))
  (bind _output_get (Variables|/Game/Blueprints/UI/ButtonPrompt.ButtonPrompt_C|SetIsInteract _asbutton_prompt IsInteract))
  (Widget|SetVisibility (Variables|/Game/Blueprints/UI/ButtonPrompt.ButtonPrompt_C|GetTextBlock_52 _asbutton_prompt) (select _output_get "Visible" "Collapsed")))