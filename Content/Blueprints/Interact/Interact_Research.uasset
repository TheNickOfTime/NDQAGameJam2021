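; Interactable research object that opens and closes a computer UI for the player.
; On BeginPlay it creates a ComputerUI widget for player controller 0 and keeps it for reuse.
; Each OnInteract call flips InUI, adding the widget to the viewport and deactivating character movement, or removing it and reactivating movement.
; Closing also re-enables input on the player controller.
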(event EventBeginPlay
  (bind _returnvalue (UserInterface|CreateWidget "/Game/Blueprints/UI/ComputerUI.ComputerUI_C" (Game|GetPlayerController 0)))
  (Variables|Default|SetUI _returnvalue))

(fn ConstructionScript
  (|CallParentFunction))

(fn OnInteract
  (bind _returnvalue (Game|GetPlayerController 0))
  (bind _returnvalue_2 (Game|GetPlayerCharacter 0))
  (bind _ui (Variables|Default|GetUI))
  (bind _charactermovement (Variables|/Script/Engine.Character|GetCharacterMovement _returnvalue_2))
  (Variables|Default|SetInUI (not (Variables|Default|GetInUI)))
  (if (Variables|Default|GetInUI)
    (UserInterface|Viewport|AddtoViewport _ui 0)
    (Components|Activation|Deactivate _charactermovement)
    (else
      (Widget|RemovefromParent _ui)
      (Input|EnableInput _returnvalue _returnvalue)
      (Components|Activation|Activate _charactermovement false))))