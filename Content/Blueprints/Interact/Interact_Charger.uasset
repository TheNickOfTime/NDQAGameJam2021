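; Interactable charger that trades one unit of the player's resource for a full charge.
; On interaction, it checks that player 0 has resource left, decrements it, sets the current charge to the maximum and plays an audio component.
; With no resource left, the interaction does nothing.
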(fn ConstructionScript
  (|CallParentFunction))

(fn OnInteract
  (bind _returnvalue (Game|GetPlayerCharacter 0))
  (bind _asplayer (Utilities|Casting|CastToPlayer _returnvalue))
  (bind _currentresource (Variables|/Game/Blueprints/Player/Player.Player_C|GetCurrentResource _asplayer))
  (if (> _currentresource 0)
    (Math|Integer|DecrementInt _currentresource
      (:%20%20
        (Variables|/Game/Blueprints/Player/Player.Player_C|SetCurrentCharge _asplayer (Math|Conversions|ToFloat(Integer) (Variables|/Game/Blueprints/Player/Player.Player_C|GetMaxCharge _asplayer)))
        (Audio|Components|Audio|Play (Variables|Default|GetAudio) 0.0)))))