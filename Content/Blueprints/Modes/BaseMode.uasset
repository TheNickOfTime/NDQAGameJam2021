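; BaseMode is a game mode that handles save, load and delete of the player's progress through a PlayerData save game in one slot.
; On BeginPlay it loads the slot, or creates a new save with charge at the player's maximum, then copies resources, charge and age to the Player and research and first-run state to itself.
; Saving gathers those values back before writing; deleting clears the slot and reloads defaults.
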(event EventBeginPlay
  (CallFunction|GetSaveData))

(event EventTick
  (params (DeltaSeconds :type Float%20%28single-precision%29)))

(fn ConstructionScript)

(fn GetSaveData
  (Utilities|FlowControl|Sequence
    (:then_0
      (bind _returnvalue (SaveGame|DoesSaveGameExist (Variables|Default|GetSaveDataSlot)))
      (if _returnvalue
        (bind _returnvalue_2 (SaveGame|LoadGamefromSlot (Variables|Default|GetSaveDataSlot)))
        (bind _asplayer_data (Utilities|Casting|CastToPlayerData _returnvalue_2))
        (Variables|Default|SetSaveData _asplayer_data)
        (else
          (bind _returnvalue_3 (SaveGame|CreateSaveGameObject "/Game/Blueprints/Save/PlayerData.PlayerData_C"))
          (bind _output_get (Variables|Default|SetSaveData _returnvalue_3))
          (Variables|/Game/Blueprints/Save/PlayerData.PlayerData_C|SetCharge _output_get (Math|Conversions|ToFloat(Integer) (Variables|/Game/Blueprints/Player/Player.Player_C|GetMaxCharge (.AsPlayer (Utilities|Casting|CastToPlayer (Game|GetPlayerCharacter 0)))))))))
    (:then_1
      (bind _asplayer (Utilities|Casting|CastToPlayer (Game|GetPlayerCharacter 0)))
      (Variables|/Game/Blueprints/Player/Player.Player_C|SetCurrentResource _asplayer (Math|Float|Truncate (Variables|/Game/Blueprints/Save/PlayerData.PlayerData_C|GetResources (Variables|Default|GetSaveData))))
      (Variables|Default|SetCurrentResearch (Variables|/Game/Blueprints/Save/PlayerData.PlayerData_C|GetResearch (Variables|Default|GetSaveData)))
      (Variables|/Game/Blueprints/Player/Player.Player_C|SetCurrentCharge _asplayer (Variables|/Game/Blueprints/Save/PlayerData.PlayerData_C|GetCharge (Variables|Default|GetSaveData)))
      (Variables|Default|SetFirstRun (Variables|/Game/Blueprints/Save/PlayerData.PlayerData_C|GetFirstRun (Variables|Default|GetSaveData)))
      (Variables|/Game/Blueprints/Player/Player.Player_C|SetCurrentAge _asplayer (Variables|/Game/Blueprints/Save/PlayerData.PlayerData_C|GetAge (Variables|Default|GetSaveData))))))

(fn SetSaveData
  (CallFunction|UpdateSaveData)
  (SaveGame|SaveGametoSlot (Variables|Default|GetSaveData) (Variables|Default|GetSaveDataSlot)))

(fn UpdateSaveData
  (bind _returnvalue (Game|GetGameMode))
  (bind _savedata (Variables|Default|GetSaveData))
  (bind _asbase_mode (Utilities|Casting|CastToBaseMode _returnvalue))
  (bind _asplayer (Utilities|Casting|CastToPlayer (Game|GetPlayerCharacter 0)))
  (Variables|/Game/Blueprints/Save/PlayerData.PlayerData_C|SetResources _savedata (Math|Conversions|ToFloat(Integer) (Variables|/Game/Blueprints/Player/Player.Player_C|GetCurrentResource _asplayer)))
  (Variables|/Game/Blueprints/Save/PlayerData.PlayerData_C|SetCharge _savedata (Variables|/Game/Blueprints/Player/Player.Player_C|GetCurrentCharge _asplayer))
  (Variables|/Game/Blueprints/Save/PlayerData.PlayerData_C|SetResearch _savedata (Variables|BaseMode_C|GetCurrentResearch _asbase_mode))
  (Variables|/Game/Blueprints/Save/PlayerData.PlayerData_C|SetAge _savedata (Variables|/Game/Blueprints/Player/Player.Player_C|GetCurrentAge _asplayer))
  (Variables|/Game/Blueprints/Save/PlayerData.PlayerData_C|SetFirstRun _savedata (Variables|BaseMode_C|GetFirstRun _asbase_mode)))

(fn DeleteSaveData
  (SaveGame|DeleteGameinSlot (Variables|Default|GetSaveDataSlot))
  (CallFunction|GetSaveData)
  (Development|PrintString "Save Data has been deleted - I hope this is what you wanted"))