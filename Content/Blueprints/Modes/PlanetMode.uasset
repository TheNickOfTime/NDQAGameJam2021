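; Game mode for a planet level that builds a randomized arena and drains the player's charge over time.
; BeginPlay caches the player, sky sphere and sun, then loads level instances from a shuffled index list at each LevelSpawnPos actor.
; Tick lowers the player's CurrentCharge by delta time scaled by Timescale.
; A day cycle that lerps horizon color and sun rotation exists but is disconnected, so it never runs.
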(event EventBeginPlay
  (|CallParentFunction)
  (|SetPlayerRef)
  (|SetLightRefs)
  (CallFunction|SetUpArena))

(event EventTick
  (params (DeltaSeconds :type Float%20%28single-precision%29))
  (CallFunction|TimePassingPlayerCharge DeltaSeconds))

(fn ConstructionScript)

(fn TimePassingPlayerCharge
  (params (delta :type Float%20%28single-precision%29))
  (bind _playerref (Variables|Default|GetPlayerRef))
  (Variables|/Game/Blueprints/Player/Player.Player_C|SetCurrentCharge _playerref (- (Variables|/Game/Blueprints/Player/Player.Player_C|GetCurrentCharge _playerref) (* delta (Variables|Default|GetTimescale)))))

(fn TimePassingDay
  (params (delta :type Float%20%28single-precision%29))
  (bind _skybox (Variables|Light|GetSkybox))
  (bind _output_get (Variables|Default|SetTimeOfDayCurrent (+ (Variables|Default|GetTimeOfDayCurrent) (* delta (Variables|Default|GetTimescale)))))
  (Variables|/Engine/EngineSky/BP_Sky_Sphere.BP_Sky_Sphere_C|SetHorizon%20color _skybox (Math|Color|Lerp(LinearColor) (Variables|Default|GetHorizonColorStart) (Variables|Default|GetHorizonColorEnd) (/ _output_get (Variables|Default|GetTimeOfDayMax))))
  (Default|RefreshMaterial _skybox)
  (Transformation|SetWorldRotation (Variables|/Script/Engine.Light|GetLightComponent (Variables|Light|GetSun)) (Math|Rotator|Lerp(Rotator) (Variables|Default|GetSunRotationStart) (Variables|Default|GetSunRotationEnd) (/ _output_get (Variables|Default|GetTimeOfDayMax))) false false))

(fn SetUpArena
  (bind _levelindex (Variables|Default|GetLevelIndex))
  (for (_ _array_index) (Variables|Default|GetLevelRefs)
    (Utilities|Array|Add _levelindex _array_index)
    (Utilities|Array|Shuffle _levelindex))
  (bind _outactors (Actor|GetAllActorsOfClass "/Game/Blueprints/Level/LevelSpawnPos.LevelSpawnPos_C"))
  (for (_array_element _array_index_2) _outactors
    (Class|LevelStreamingDynamic|LoadLevelInstancebySoftObjectPtr (Utilities|Array|Get(acopy) (Variables|Default|GetLevelRefs) (Utilities|Array|Get(acopy) (Variables|Default|GetLevelIndex) _array_index_2)) (Transformation|GetActorLocation _array_element) "0, 0, 0")))