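; Mode is a player-related Blueprint that drains the player's CurrentCharge over time.
; On BeginPlay it casts the first player character to Player and caches the reference.
; Every Tick passes the frame delta to TimePassing, which subtracts it, scaled by Timescale, from that charge, with no clamping in this graph.
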(event EventBeginPlay
  (bind _asplayer (Utilities|Casting|CastToPlayer (Game|GetPlayerCharacter 0)))
  (Variables|Default|SetPlayerRef _asplayer))

(event EventTick
  (params (DeltaSeconds :type Float%20%28single-precision%29))
  (CallFunction|TimePassing DeltaSeconds))

(fn ConstructionScript)

(fn TimePassing
  (params (delta :type Float%20%28single-precision%29))
  (bind _playerref (Variables|Default|GetPlayerRef))
  (Variables|/Game/Blueprints/Player/Player.Player_C|SetCurrentCharge _playerref (- (Variables|/Game/Blueprints/Player/Player.Player_C|GetCurrentCharge _playerref) (* delta (Variables|Default|GetTimescale)))))