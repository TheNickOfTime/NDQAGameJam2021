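; Player controller that turns input into actions on the controlled Player pawn.
; It caches the pawn at BeginPlay, passes the vertical and horizontal axes to its Move every Tick, and forwards Jump and Interact presses.
; Releasing Tab calls DeleteSaveData on the BaseMode game mode.
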(event EventTick
  (params (DeltaSeconds :type Float%20%28single-precision%29))
  (Default|Move (Variables|Default|GetPlayerRef) (Math|Vector|MakeVector (Input|AxisValues|GetVertical) (Input|AxisValues|GetHorizontal) 0.0)))

(event EventBeginPlay
  (bind _asplayer (Utilities|Casting|CastToPlayer (Pawn|GetControlledPawn)))
  (Variables|Default|SetPlayerRef _asplayer))

(event Input|ActionEvents|InputActionJump
  (params (Key :type Key%20Structure :default "None"))
  (:Pressed
    (Default|Jumping (Variables|Default|GetPlayerRef))))

(event Input|ActionEvents|InputActionInteract
  (params (Key :type Key%20Structure :default "None"))
  (:Pressed
    (Default|Interact (Variables|Default|GetPlayerRef))))

(event Input|KeyboardEvents|Tab
  (params (Key :type Key%20Structure :default "None"))
  (:Released
    (bind _asbase_mode (Utilities|Casting|CastToBaseMode (Game|GetGameMode)))
    (Default|DeleteSaveData _asbase_mode)))

(fn ConstructionScript)