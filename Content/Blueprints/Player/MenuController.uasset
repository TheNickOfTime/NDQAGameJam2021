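; MenuController is the player controller for the main menu, driven by gamepad face buttons.
; On BeginPlay it creates the MainMenu widget and adds it to the viewport.
; The bottom button plays a start sound, then opens the TestSpaceship level after a delay.
; The left button toggles the widget's ShowCredits flag with a blip, while the right button plays a blip and quits after a short delay.
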(event EventBeginPlay
  (bind _returnvalue (UserInterface|CreateWidget "/Game/Blueprints/UI/MainMenu.MainMenu_C" self))
  (bind _output_get (Variables|Default|SetUI _returnvalue))
  (UserInterface|Viewport|AddtoViewport _output_get 0))

(event Input|GamepadEvents|GamepadFaceButtonBottom
  (params (Key :type Key%20Structure :default "None"))
  (:Released
    (Audio|PlaySound2D "/Game/Audio/SFX/GJ_PressStart.GJ_PressStart" 1.0 1.0 0.5 0 0)
    (Utilities|FlowControl|Delay 5.0)
    (Game|OpenLevel(byObjectReference) "/Game/Levels/TestSpaceship.TestSpaceship")))

(event Input|GamepadEvents|GamepadFaceButtonTop
  (params (Key :type Key%20Structure :default "None")))

(event Input|GamepadEvents|GamepadFaceButtonLeft
  (params (Key :type Key%20Structure :default "None"))
  (bind _ui (Variables|Default|GetUI))
  (:Released
    (Variables|/Game/Blueprints/UI/MainMenu.MainMenu_C|SetShowCredits _ui (not (Variables|/Game/Blueprints/UI/MainMenu.MainMenu_C|GetShowCredits _ui)))
    (Audio|PlaySound2D "/Game/Audio/SFX/UI_Nav_Blips/UI_Blips_High.UI_Blips_High" 1.0 1.0 0.0 0 0)))

(event Input|GamepadEvents|GamepadFaceButtonRight
  (params (Key :type Key%20Structure :default "None"))
  (:Released
    (Audio|PlaySound2D "/Game/Audio/SFX/UI_Nav_Blips/UI_Blips_Low.UI_Blips_Low" 1.0 1.0 0.0 0 0)
    (Utilities|FlowControl|Delay 1.0)
    (Game|QuitGame 0 "Quit" false)))

(fn ConstructionScript)