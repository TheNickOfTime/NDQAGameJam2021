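; Player character Blueprint that exposes movement, jump and interact actions and owns the on-screen HUD.
; On BeginPlay it creates the HUD widget, hands it a self reference, then fills the current charge to its maximum.
; Landing triggers force feedback and camera shake, and Interact forwards to the current interactable.
; SetAnimState is an unfinished stub that only checks for falling.
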(event EventOnLanded
  (params (Hit :type Hit%20Result%20Structure%20%28by%20ref%29))
  (bind _returnvalue (Game|GetPlayerController 0))
  (Game|Feedback|ClientPlayForceFeedback _returnvalue "/Game/Blueprints/Rumbles/Land.Land" "None" false false false)
  (Game|Feedback|ClientStartCameraShake _returnvalue "/Game/Blueprints/CameraShakes/LandShake.LandShake_C" 1.0 "CameraLocal" "0, 0, 0"))

(event EventBeginPlay
  (|CreateHUD
    (:output
      (Variables|Health|SetCurrentCharge (Math|Conversions|ToFloat(Integer) (Variables|Health|GetMaxCharge))))))

(fn ConstructionScript)

(fn Move
  (params (Direction :type Vector))
  (Pawn|Input|AddMovementInput Direction 1.0 false))

(fn Jumping
  (Character|Jump))

(fn Interact
  (if (!= (Variables|Default|GetCurrentInteract) 0)
    (Default|OnInteract (Variables|Default|GetCurrentInteract))))

(fn SetAnimState
  (if (AI|Components|NavMovement|IsFalling (Variables|Character|GetCharacterMovement))
    _))